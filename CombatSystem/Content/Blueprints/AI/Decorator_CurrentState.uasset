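; Behavior Tree decorator that gates a branch on the current state of a character stored in the Blackboard.
; It reads the actor from the CharacterToCheck key, casts it to CSCharacter and passes only when its CurrentState equals StateToCheck.
; An invalid actor or failed cast fails the check.
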(fn PerformConditionCheckAI
  (params (OwnerController :type AI%20Controller%20Object%20Reference) (ControlledPawn :type Pawn%20Object%20Reference))
  (bind _charactertocheck (Variables|Default|GetCharacterToCheck))
  (bind _returnvalue (AI|BehaviorTree|GetBlackboardValueasActor _charactertocheck))
  (Utilities|IsValid _returnvalue
    (:Is%20Valid
      (bind _ascscharacter (Utilities|Casting|CastToCSCharacter _returnvalue)
        (:then
          (return (== (Math|Conversions|ToInteger(Byte) (Variables|/Script/CombatSystem.CSCharacter|GetCurrentState _ascscharacter)) (Math|Conversions|ToInteger(Byte) (Variables|Default|GetStateToCheck)))))
        (:CastFailed
          (return false))))
    (:Is%20Not%20Valid
      (return false))))