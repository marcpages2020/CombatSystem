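; Behavior tree task that makes an AI-controlled CSCharacter dodge in a randomized direction.
; It fetches the character's DODGE state as BP_StateDodge, sets its direction, then requests that state.
; The direction is the flattened backward vector rotated around Z by a random angle up to 120 degrees either side.
; It finishes successfully right after the request without waiting for the dodge, and calls FinishAbort if a cast or state lookup fails.
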(event EventReceiveExecuteAI
  (params (OwnerController :type AI%20Controller%20Object%20Reference) (ControlledPawn :type Pawn%20Object%20Reference))
  (bind _ascscharacter (Utilities|Casting|CastToCSCharacter ControlledPawn)
    (:then
      (bind _output_get (Variables|Default|SetCharacter _ascscharacter))
      (bind _returnvalue (Class|CSCharacter|GetCharacterState _output_get "DODGE"))
      (Utilities|IsValid _returnvalue
        (:Is%20Valid
          (bind _asbp_state_dodge (Utilities|Casting|CastToBP_StateDodge _returnvalue)
            (:then
              (bind _returnvalue_2 (CallFunction|CalculateDodgeDirection))
              (Class|CSCharacterStateDodge|SetDodgeDirection _asbp_state_dodge _returnvalue_2)
              (Class|CSCharacter|RequestState _output_get "DODGE")
              (Development|PrintString "Dodge Requested" true true "(R=1.000000,G=0.846875,B=0.000000,A=1.000000)" 1.0)
              (AI|BehaviorTree|FinishExecute true))
            (:CastFailed
              (Development|PrintString "Could not cast state" true true "(R=0.427083,G=0.006833,B=0.000000,A=1.000000)")
              (Class|BTTaskBlueprintBase|FinishAbort))))
        (:Is%20Not%20Valid
          (Development|PrintString "No DodgeState" true true "(R=0.427083,G=0.006833,B=0.000000,A=1.000000)")
          (Class|BTTaskBlueprintBase|FinishAbort))))
    (:CastFailed
      (Class|BTTaskBlueprintBase|FinishAbort))))

(fn CalculateDodgeDirection
  (return (Math|Vector|RotateVectorAroundAxis (* (Transformation|GetActorForwardVector (Variables|Default|GetCharacter)) "-1.000000,-1.000000,0") (Math|Random|RandomFloatinRange 1.2e+02 -1.2e+02) (Math|Vector|MakeVector 0.0 0.0 1.0))))