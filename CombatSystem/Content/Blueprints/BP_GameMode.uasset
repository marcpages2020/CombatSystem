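; BP_GameMode is a game mode that spawns AI enemies and reacts to wave state changes.
; SpawnNewEnemy runs the EQS_FindSpawnLocation query, picking at random from the best 25% of results.
; On success, it spawns BP_Enemy_AI at each returned location, adjusting for collisions or skipping if blocked, and draws debug spheres there.
; WaveStateChanged only prints the new state on screen for debugging.
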(event Custom|OnQueryFinishedEvent_Event_0
  (params (QueryInstance :type Env%20Query%20Instance%20Blueprint%20Wrapper%20Object%20Reference) (QueryStatus :type EEnvQueryStatus%20Enum :default "Processing"))
  (switch Utilities|FlowControl|Switch|SwitchonEEnvQueryStatus QueryStatus
    (:Success
      (bind _resultlocations (AI|EQS|GetQueryResultsasLocations QueryInstance))
      (for _array_element _resultlocations
        (Rendering|Debug|DrawDebugSphere _array_element 5e+01 12 "(R=1.000000,G=0.928322,B=0.000000,A=1.000000)" 2.0 2.0)
        (Game|SpawnActorfromClass "/Game/Blueprints/AI/BP_Enemy_AI.BP_Enemy_AI_C" (Math|Transform|MakeTransform _array_element) "AdjustIfPossibleButDontSpawnIfColliding" 0 0)))))

(event EventSpawnNewEnemy
  (bind _returnvalue (AI|EQS|RunEQSQuery "/Game/Blueprints/AI/EnvironmentQueries/EQS_FindSpawnLocation.EQS_FindSpawnLocation" self "RandomBest25Pct"))
  (EventDispatchers|AssignOnQueryFinishedEvent _returnvalue (delegate Custom|OnQueryFinishedEvent_Event_0)))

(event EventWaveStateChanged
  (params (NewState :type EWaveState%20Enum :default "WaitingToStart") (OldState :type EWaveState%20Enum :default "WaitingToStart"))
  (Development|PrintString (Utilities|String|EnumtoString NewState) true true "(R=1.000000,G=0.000000,B=0.615759,A=1.000000)" 5.0))

(fn ConstructionScript)