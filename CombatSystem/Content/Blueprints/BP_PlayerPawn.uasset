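; BP_PlayerPawn is a player pawn Blueprint with startup setup and a state debug readout.
; On BeginPlay it caches itself cast to CSCharacter, then constructs a locked-target indicator widget and stores it if valid; the AddToViewport call is disconnected.
; Tick prints CurrentState on screen, using DeltaSeconds as the duration so the message refreshes each frame.
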(event EventTick
  (params (DeltaSeconds :type Float%20%28single-precision%29))
  (Utilities|FlowControl|Sequence
    (:then_0
      (Development|PrintString (Utilities|String|EnumtoString (Variables|Default|GetCurrentState self)) true false "(R=0.000000,G=0.660000,B=1.000000,A=1.000000)" DeltaSeconds))))

(event EventBeginPlay
  (Utilities|FlowControl|Sequence
    (:then_0
      (bind _ascscharacter (Utilities|Casting|CastToCSCharacter self))
      (Variables|Default|SetCharacterReference _ascscharacter))
    (:then_1
      (bind _returnvalue (Game|ConstructObjectfromClass "/Game/Blueprints/UI/WBP_LockedTargetIndicator.WBP_LockedTargetIndicator_C" self))
      (Utilities|IsValid 0
        (:Is%20Valid
          (Variables|Default|SetLockedTargetIndicator _returnvalue))))))

(fn ConstructionScript)